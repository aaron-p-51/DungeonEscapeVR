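; BP_VRPlayerCharacter is the VR player character Blueprint, handling camera fade for collisions.
; Collision start and stop events play and reverse a timeline, whose alpha drives a manual camera fade to the collision fade color on each update.
; An unconnected graph, which never runs, would disable capsule collision and teleport VRCenter to the first actor tagged PauseLocation.
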(event EventCollisionStartCameraFade
  (bind _camerafadealpha (Timeline|CameraFadeOutTimeline Play)
    (:Update
      (Class|PlayerCameraManager|SetManualCameraFade (Game|GetPlayerCameraManager 0) _camerafadealpha (Class|DVRPlayerCharacter|GetCameraCollisionFadeColor) false))))

(event EventCollisionStopCameraFade
  (bind _camerafadealpha (Timeline|CameraFadeOutTimeline Reverse)
    (:Update
      (Class|PlayerCameraManager|SetManualCameraFade (Game|GetPlayerCameraManager 0) _camerafadealpha (Class|DVRPlayerCharacter|GetCameraCollisionFadeColor) false))))

(event Input|ActionEvents|InputActionPause
  (params (Key :type Key%20Structure :default "None")))

(fn ConstructionScript)