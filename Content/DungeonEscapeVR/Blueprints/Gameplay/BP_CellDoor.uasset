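; BP_CellDoor is a dungeon cell door actor that opens and closes with sound and rubble effects.
; OpenCellDoor and CloseCellDoor each play a timeline that drives the door height and fires completion events.
; Timeline event tracks time the movement and impact sounds, with the opening impact played when the timeline finishes.
; An opening event track also spawns rubble emitters at three component locations cached on BeginPlay.
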(event EventBeginPlay
  (bind _rubblespawnlocations (Variables|Default|GetRubbleSpawnLocations))
  (Utilities|Array|Add _rubblespawnlocations (Transformation|GetWorldLocation (Variables|Default|GetRubbleFXSpawnLocation01)))
  (Utilities|Array|Add _rubblespawnlocations (Transformation|GetWorldLocation (Variables|Default|GetRubbleFXSpawnLocation02)))
  (Utilities|Array|Add _rubblespawnlocations (Transformation|GetWorldLocation (Variables|Default|GetRubbleFXSpawnLocation03))))

(event Collision|EventActorBeginOverlap
  (params (OtherActor :type Actor%20Object%20Reference)))

(event EventOpenCellDoor
  (bind _returnvalue (Transformation|GetActorLocation))
  (bind _celldoorheight (Timeline|OpenDoorTimeline PlayFromStart)
    (:Update
      (Class|DCellDoor|OnUpdateCellDoorHeight _celldoorheight))
    (:Finished
      (Audio|PlaySoundatLocation "/Game/DungeonEscapeVR/Audio/Cues/S_CellDoorOpenImpact_Cue.S_CellDoorOpenImpact_Cue" _returnvalue "0, 0, 0" 1.0 1.0 0.0 0 0 0)
      (Class|DCellDoor|OnFinishCellDoorOpened))
    (:VFX%20Track
      (CallFunction|SpawnRubbleFX))
    (:SFX%20Track
      (Audio|PlaySoundatLocation "/Game/DungeonEscapeVR/Audio/Cues/S_CellDoorOpen_Cue.S_CellDoorOpen_Cue" _returnvalue "0, 0, 0" 1.0 1.0 0.0 0 0 0))))

(event EventCloseCellDoor
  (bind _returnvalue (Transformation|GetActorLocation))
  (bind _closecelldoorheight (Timeline|CloseDoorTimeline PlayFromStart)
    (:Update
      (Class|DCellDoor|OnUpdateCellDoorHeight _closecelldoorheight))
    (:Finished
      (Class|DCellDoor|OnFinishedCellDoorClosed))
    (:SFX%20DoorClose
      (Audio|PlaySoundatLocation "/Game/DungeonEscapeVR/Audio/Cues/S_CellDoorClose_Cue.S_CellDoorClose_Cue" _returnvalue "0, 0, 0" 1.0 1.0 0.0 0 0 0))
    (:SFX_DoorCloseImpact
      (Audio|PlaySoundatLocation "/Game/DungeonEscapeVR/Audio/Cues/S_CellDoorCloseImpact_Cue.S_CellDoorCloseImpact_Cue" _returnvalue "0, 0, 0" 1.0 1.0 0.0 0 0 0))))

(fn ConstructionScript)

(fn SpawnRubbleFX
  (for _array_element (Variables|Default|GetRubbleSpawnLocations)
    (Effects|SpawnEmitteratLocation "/Game/DungeonEscapeVR/FX/P_CellDoorRuble.P_CellDoorRuble" _array_element)))